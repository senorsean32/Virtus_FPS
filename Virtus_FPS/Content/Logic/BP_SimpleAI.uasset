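; BP_SimpleAI is a basic AI pawn that wanders, chases the player soldier and can be shot dead.
; Tick uses a Delay to throttle random roaming; PawnSensing switches it to chasing, clearing the sighting and setting walk speed when the move ends.
; BeenShot reduces health, spawns impact effects, briefly flags hits and sends it toward the player.
; Death spawns an enlarged effect, stops movement and disables collision.
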(event OnSeePawn(PawnSensing)
  (params (Pawn :type Pawn%20Object%20Reference))
  (Variables|Default|SetCanSeePlayer true)
  (bind _asbp_char_soldier (Utilities|Casting|CastToBP_Char_Soldier Pawn))
  (if (not (Variables|Default|GetDead))
    (AI|AIMoveTo self "0, 0, 0" _asbp_char_soldier 5.0 false
      (:OnSuccess
        _)
      (:OnFail
        _))
    (Variables|Default|SetCanSeePlayer false)
    (Variables|/Script/Engine.CharacterMovementComponent|SetMaxWalkSpeed (Variables|Character|GetCharacterMovement) 3e+02)))

(event Custom|BeenShot
  (params (HitInfo :type Hit%20Result%20Structure))
  (bind _impactpoint (Collision|BreakHitResult HitInfo))
  (Variables|Default|SetHealth (- (Variables|Default|GetHealth) 0.65))
  (if (< (Variables|Default|GetHealth) 0.1)
    (bind _returnvalue (Effects|SpawnEmitteratLocation "/Game/InfinityBladeEffects/Effects/FX_Mobile/Impacts/P_Impact_Shield_Fire.P_Impact_Shield_Fire" _impactpoint))
    (Transformation|SetWorldScale3D _returnvalue "3.000000,3.000000,3.000000")
    (Variables|Default|SetDead true)
    (if (Variables|Default|GetDead)
      (AI|Navigation|StopMovement (Pawn|GetController))
      (Collision|SetActorEnableCollision false))
    (else
      (Variables|Default|SetHit true)
      (Development|PrintString "AI: Hit" true false)
      (Effects|SpawnEmitteratLocation "/Game/InfinityBladeEffects/Effects/FX_Mobile/Impacts/P_Impact_Shield_Fire.P_Impact_Shield_Fire" _impactpoint)
      (bind _asbp_char_soldier (Utilities|Casting|CastToBP_Char_Soldier (Game|GetPlayerCharacter 0)))
      (AI|AIMoveTo self "0, 0, 0" _asbp_char_soldier 5.0 false
        (:then
          (Utilities|FlowControl|Delay 0.1)
          (Variables|Default|SetHit false))))))

(event EventBeginPlay)

(event EventTick
  (params (DeltaSeconds :type Float%20%28single-precision%29))
  (if (Variables|Default|GetDead)
    (AI|Navigation|StopMovement (Pawn|GetController))
    (else
      (Utilities|FlowControl|Delay 3.0)
      (if (not (Variables|Default|GetCanSeePlayer))
        (AI|AIMoveTo self (.RandomLocation (AI|Navigation|GetRandomReachablePointinRadius (Transformation|GetActorLocation) 5e+03)) 0 5.0 false)))))

(fn ConstructionScript)