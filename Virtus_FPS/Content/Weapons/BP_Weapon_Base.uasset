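; Base weapon Blueprint for the player soldier, handling ammo, fire effects and reloading.
; BeginPlay caches the player's BP_Char_Soldier and fills the clip; Fire decrements ammo and plays rifle sound plus a particle at the soldier's Muzzle socket.
; Reload either discards leftover rounds (hardcore) or tops up from reserve, generally flagging the soldier as reloading.
; Projectile spawning and an alternate muzzle flash are disconnected, so Fire launches nothing.
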(event Custom|Fire
  (bind _charsoldierbp (Variables|Components|GetCharSoldierBP))
  (bind _skeletalmesh (Variables|/Game/Logic/BP_Char_Soldier.BP_Char_Soldier_C|GetSkeletalMesh _charsoldierbp))
  (Variables|Default|SetAmmo (- (Variables|Default|GetAmmo) 1))
  (bind _returnvalue (Effects|SpawnEmitteratLocation "/Game/InfinityBladeEffects/Effects/FX_Combat_Base/Notifies/P_FootSteps_Run.P_FootSteps_Run" (Transformation|GetSocketLocation _skeletalmesh "Muzzle") (Transformation|GetSocketRotation _skeletalmesh "Muzzle")))
  (Transformation|SetWorldScale3D _returnvalue "0.500000,0.500000,0.500000")
  (Audio|PlaySound2D "/Game/Weapons/AK47/Aud_Rifle_Fire.Aud_Rifle_Fire"))

(event EventBeginPlay
  (bind _asbp_char_soldier (Utilities|Casting|CastToBP_Char_Soldier (Game|GetPlayerCharacter 0)))
  (Variables|Components|SetCharSoldierBP _asbp_char_soldier)
  (Variables|Default|SetAmmo (Variables|Default|GetClipSize)))

(fn ConstructionScript)

(fn Reload
  (params (HardcoreReload :type Boolean))
  (if HardcoreReload
    ;[1 1 1] Hardcore Reload system (unused ammo gets discarded on reload)
    (if (not (== (Variables|Default|GetAmmo) (Variables|Default|GetClipSize)))
      (if (> (Variables|Default|GetMaxAmmo) (Variables|Default|GetClipSize))
        (Variables|Default|SetAmmo (Variables|Default|GetClipSize))
        (Variables|Default|SetMaxAmmo (- (Variables|Default|GetMaxAmmo) (Variables|Default|GetClipSize)))
        (bind _output_get (Variables|/Game/Logic/BP_Char_Soldier.BP_Char_Soldier_C|SetIsReloading (Variables|Components|GetCharSoldierBP) true))
        (return (or _output_get (stale _output_get_2)))
        (else
          (Variables|Default|SetAmmo (Variables|Default|GetMaxAmmo))
          (Variables|Default|SetMaxAmmo 0))))
    (else
      ;[1 1 1] Standard Gaming reload system
      (if (and (> (Variables|Default|GetMaxAmmo) 0) (< (Variables|Default|GetAmmo) (Variables|Default|GetClipSize)))
        (LocalVariables|Set_AmmoDifference (- (Variables|Default|GetClipSize) (Variables|Default|GetAmmo)))
        (Variables|Default|SetAmmo (+ (Variables|Default|GetAmmo) (LocalVariables|Get_AmmoDifference)))
        (Variables|Default|SetMaxAmmo (Math|Integer|Clamp(Integer) (- (Variables|Default|GetMaxAmmo) (LocalVariables|Get_AmmoDifference)) 0 (Variables|Default|GetMaxAmmo)))
        (bind _output_get_2 (Variables|/Game/Logic/BP_Char_Soldier.BP_Char_Soldier_C|SetIsReloading (Variables|Components|GetCharSoldierBP) true))
        (return (or _output_get _output_get_2))))))